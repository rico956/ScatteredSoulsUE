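; BP_DragPuzzle is a trigger actor that gates a door behind a drag puzzle widget.
; Box overlap by ThirdPersonCharacter pauses the game, shows WBP_DragFrom with mouse input and hands the widget to the player character.
; On the widget's finished event, it restores play, removes the trigger and slides Door with sound via a Delay-looped VInterpToConstant.
; The whole actor destroys itself once the door reaches its target height.
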(event OnComponentBeginOverlap(Box)
  (params (OverlappedComponent :type Primitive%20Component%20Object%20Reference) (OtherActor :type Actor%20Object%20Reference) (OtherComp :type Primitive%20Component%20Object%20Reference) (OtherBodyIndex :type Integer) (bFromSweep :type Boolean) (SweepResult :type Hit%20Result%20Structure%20%28by%20ref%29))
  (bind _returnvalue (Game|GetPlayerController 0))
  (Utilities|Casting|CastToThirdPersonCharacter OtherActor)
  (Game|SetGamePaused true)
  (bind _returnvalue_2 (UserInterface|CreateWidget "/Game/UI/Puzzle/WBP_DragFrom.WBP_DragFrom_C"))
  (bind _output_get (Variables|Default|SetPuzzleWidget _returnvalue_2))
  (UserInterface|Viewport|AddtoViewport _output_get 0)
  (bind _asthird_person_character (Utilities|Casting|CastToThirdPersonCharacter (Game|GetPlayerCharacter 0)))
  (Variables|/Game/ThirdPersonBP/Blueprints/ThirdPersonCharacter.ThirdPersonCharacter_C|SetDragWidget _asthird_person_character (Variables|Default|GetPuzzleWidget))
  (Variables|/Script/Engine.PlayerController|SetbShowMouseCursor _returnvalue true)
  (Input|SetInputModeGameandUI _returnvalue 0 "DoNotLock" false)
  (EventDispatchers|BindEventtoFinishedPuzzle (Variables|Default|GetPuzzleWidget) (delegate Custom|FinishedPuzzle)))

(event Custom|FinishedPuzzle
  (bind _returnvalue (Game|GetPlayerController 0))
  (bind _door (Variables|Default|GetDoor))
  (Variables|/Script/Engine.PlayerController|SetbShowMouseCursor _returnvalue false)
  (Input|SetInputModeGameOnly _returnvalue)
  (Widget|RemovefromParent (Variables|Default|GetPuzzleWidget))
  (Game|SetGamePaused false)
  (Components|DestroyComponent (Variables|Default|GetBox))
  (Variables|Default|SetEndPosition (* (Variables|/Script/Engine.SceneComponent|GetRelativeLocation _door) "1.000000,1.000000,-1.100000"))
  (bind _returnvalue_2 (Audio|SpawnSoundatLocation "/Game/sounds/stone_gates_opening.stone_gates_opening" (Transformation|GetWorldLocation _door) "0, 0, 0" 1.0 1.0 0.0 0 0))
  (Variables|Default|SetDoorSound _returnvalue_2)
  (Transformation|SetRelativeLocation (Variables|Default|GetDoor) (Math|Interpolation|VInterptoConstant (Variables|/Script/Engine.SceneComponent|GetRelativeLocation (Variables|Default|GetDoor)) (Variables|Default|GetEndPosition) (Utilities|Time|GetWorldDeltaSeconds) (Variables|Default|GetOpenDoorSpeed)) false false :!label _label)
  (if (Math|Float|NearlyEqual(Float) (.Z (Math|Vector|BreakVector (Math|Interpolation|VInterptoConstant (Variables|/Script/Engine.SceneComponent|GetRelativeLocation (Variables|Default|GetDoor)) (Variables|Default|GetEndPosition) (Utilities|Time|GetWorldDeltaSeconds) (Variables|Default|GetOpenDoorSpeed)))) (.z (Variables|Default|GetEndPosition)) 1.0)
    (Audio|Components|Audio|Stop (Variables|Default|GetDoorSound))
    (Components|DestroyComponent (Variables|Default|GetDoorSound))
    (Actor|DestroyActor)
    (else
      (Utilities|FlowControl|Delay 0.01)
      (goto _label))))

(fn ConstructionScript)